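; BP_RaftN_Spline moves its Character component along a Spline component at a set speed.
; Each Tick advances the travelled distance and applies the spline's local transform to Character, lowered in Z and yaw-corrected with fixed offsets while keeping its scale.
; When IsLooped is set, the distance resets to zero after passing the spline's end, restarting the path.
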(event EventTick
  (params (DeltaSeconds :type Float%20%28single-precision%29))
  (Variables|Default|SetSplineDistance (+ (* DeltaSeconds (Variables|Default|GetSplineSpeed)) (Variables|Default|GetSplineDistance)))
  (Transformation|SetRelativeTransform (Variables|Default|GetCharacter) (Math|Transform|MakeTransform (Math|Vector|MakeVector (.x (.location (Spline|GetTransformatDistanceAlongSpline (Variables|Default|GetSpline) (Variables|Default|GetSplineDistance) "Local" false))) (.y (.location (Spline|GetTransformatDistanceAlongSpline (Variables|Default|GetSpline) (Variables|Default|GetSplineDistance) "Local" false))) (- (.z (.location (Spline|GetTransformatDistanceAlongSpline (Variables|Default|GetSpline) (Variables|Default|GetSplineDistance) "Local" false))) 9e+01)) (Math|Rotator|MakeRotator (.roll (.rotation (Spline|GetTransformatDistanceAlongSpline (Variables|Default|GetSpline) (Variables|Default|GetSplineDistance) "Local" false))) (.pitch (.rotation (Spline|GetTransformatDistanceAlongSpline (Variables|Default|GetSpline) (Variables|Default|GetSplineDistance) "Local" false))) (- (.yaw (.rotation (Spline|GetTransformatDistanceAlongSpline (Variables|Default|GetSpline) (Variables|Default|GetSplineDistance) "Local" false))) 9e+01)) (Variables|/Script/Engine.SceneComponent|GetRelativeScale3D (Variables|Default|GetCharacter))) false false)
  (if (Variables|Default|GetIsLooped)
    (if (> (Variables|Default|GetSplineDistance) (Spline|GetSplineLength (Variables|Default|GetSpline)))
      (Variables|Default|SetSplineDistance 0.0))))

(fn ConstructionScript)