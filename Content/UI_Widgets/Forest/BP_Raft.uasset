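; BP_Raft is a raft actor that travels along a spline path in the level.
; On BeginPlay it finds a BP_RaftPath actor and starts the Move timeline, with play rate set to the inverse of TimeComplete.
; Each timeline update maps MoveT to a distance along the spline and sets the raft's world location and rotation to match that point.
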(event Custom|MoveObj
  (bind _pathref (Variables|Default|GetPathRef))
  (bind _spline (Variables|/Game/UI_Widgets/Forest/BP_RaftPath.BP_RaftPath_C|GetSpline _pathref))
  (Components|Timeline|SetPlayRate (Variables|Default|GetMove) (/ 1.0 (Variables|Default|GetTimeComplete)))
  (bind _movet (Timeline|Move Play)
    (:Update
      (Transformation|SetActorTransform (Math|Transform|MakeTransform (Spline|GetLocationatDistanceAlongSpline _spline (Math|Float|Lerp 0.0 (Spline|GetSplineLength (Variables|/Game/UI_Widgets/Forest/BP_RaftPath.BP_RaftPath_C|GetSpline (Variables|Default|GetPathRef))) _movet) "World") (Spline|GetRotationatDistanceAlongSpline _spline (Math|Float|Lerp 0.0 (Spline|GetSplineLength (Variables|/Game/UI_Widgets/Forest/BP_RaftPath.BP_RaftPath_C|GetSpline (Variables|Default|GetPathRef))) _movet) "World") "1.000000,1.000000,1.000000")))))

(event EventBeginPlay
  (bind _returnvalue (Actor|GetActorOfClass "/Game/UI_Widgets/Forest/BP_RaftPath.BP_RaftPath_C"))
  (Variables|Default|SetPathRef _returnvalue)
  (CallFunction|MoveObj))

(fn ConstructionScript)